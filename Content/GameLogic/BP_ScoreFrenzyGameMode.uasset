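; Game mode for Score Frenzy that tracks a score and scales AI difficulty with it.
; Adding or subtracting score re-evaluates two thresholds to pick Easy, Medium or Hard.
; Each change then pushes the difficulty enum into the AI controller blackboard of every BP_Character_VariantBase actor, found with GetAllActorsOfClass.
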(fn `AddScore`
  (params (Amount :type Integer))
  (set `self.Score` (+ Amount (`self.Score`)))
  (`self.UpdateDifficultyFromScore`)
  (`self.PropagateDifficultyToAllAI`))

(fn `PropagateDifficultyToAllAI`
  (bind _outactors (`GameplayStatics.GetAllActorsOfClass` "/Game/Characters/AICharacter/Variants/BP_Character_VariantBase.BP_Character_VariantBase_C"))
  (for _array_element _outactors
    (`BlackboardComponent.SetValueAsEnum` (`AIBlueprintHelperLibrary.GetBlackboard` (`Pawn.GetController` _array_element)) (`self.Difficulty Mode`) (`self.DifficultyMode`))))

(fn `SubtractScore`
  (params (Amout :type Integer))
  (set `self.Score` (- (`self.Score`) Amout))
  (`self.UpdateDifficultyFromScore`)
  (`self.PropagateDifficultyToAllAI`))

(fn `UpdateDifficultyFromScore`
  (if (>= (`self.Score`) (`self.MediumToHardThreshold`))
    (set `self.DifficultyMode` "Hard")
    (elif (>= (`self.Score`) (`self.EasyToMediumThreshold`))
      (set `self.DifficultyMode` "Medium")
      (else
        (set `self.DifficultyMode` "Easy")))))

(fn `UserConstructionScript`)