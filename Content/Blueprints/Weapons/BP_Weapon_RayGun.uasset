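; Ray gun weapon pickup that equips itself on the third-person character when they overlap its sphere.
; It destroys any weapon the character holds, snaps onto the weapon socket and registers as the current weapon.
; It then tells its owning weapon spawner to respawn a weapon and disables its own collision, both only if that owner cast succeeds.
; No firing logic is present.
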(event `self.Sphere.OnComponentBeginOverlap`
  (params (OverlappedComponent :type "PrimitiveComponent Object Reference") (OtherActor :type "Actor Object Reference") (OtherComp :type "PrimitiveComponent Object Reference") (OtherBodyIndex :type Integer) (bFromSweep :type Boolean) (SweepResult :type "HitResult Structure (by ref)"))
  (bind _asbp_third_person_character (cast `/Game/Blueprints/Weapons/Characters/Player/BP_ThirdPersonCharacter` OtherActor))
  (bind _currentweapon (`/Game/Blueprints/Weapons/Characters/Player/BP_ThirdPersonCharacter.CurrentWeapon` _asbp_third_person_character))
  (`/Engine/EditorBlueprintResources/StandardMacros.IsValid` _currentweapon
    (:`Is Valid`
      (`self.K2_DestroyActor` _currentweapon))
    (:`Is Not Valid`
      _))
  (`self.K2_AttachToComponent` (`/Game/Blueprints/Weapons/Characters/Player/BP_ThirdPersonCharacter.WeaponSocket` _asbp_third_person_character) "Weapon Socket" "SnapToTarget" "SnapToTarget" "KeepWorld" false)
  (set `/Game/Blueprints/Weapons/Characters/Player/BP_ThirdPersonCharacter.CurrentWeapon` self _asbp_third_person_character)
  (set `/Game/Blueprints/Weapons/Characters/Player/BP_ThirdPersonCharacter.HasWeapon` true _asbp_third_person_character)
  (bind _asbp_weapon_spawner (cast `/Game/Blueprints/Weapons/BP_WeaponSpawner` (`self.GetOwner`)))
  (`/Game/Blueprints/Weapons/BP_WeaponSpawner.RespawnWeapon` _asbp_weapon_spawner null)
  (`self.SetActorEnableCollision` false))

(fn `UserConstructionScript`)