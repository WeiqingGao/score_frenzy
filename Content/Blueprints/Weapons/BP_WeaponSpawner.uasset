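; Weapon spawner actor that keeps a weapon of a configured class available at its own location.
; On BeginPlay it spawns the weapon at its transform, owns it and binds to its destroyed event.
; When that weapon is destroyed, it waits for the respawn time, spawns a replacement and rebinds, repeating the cycle indefinitely.
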(event `self.ReceiveBeginPlay`
  (bind _returnvalue (`|SpawnActorFromClass` (`self.WeaponClass`) (`self.GetTransform`) "Undefined" "MultiplyWithRoot" self null))
  (set `self.CurrentWeapon` _returnvalue)
  (add `self.OnDestroyed` (`self.CurrentWeapon`) (delegate `RespawnWeapon`)))

(event `RespawnWeapon` :!signature `self.OnDestroyed`
  (params (DestroyedActor :type "Actor Object Reference"))
  (`KismetSystemLibrary.Delay` (`self.RespawnTime`))
  (bind _returnvalue (`|SpawnActorFromClass` (`self.WeaponClass`) (`self.GetTransform`) "Undefined" "MultiplyWithRoot" self null))
  (set `self.CurrentWeapon` _returnvalue)
  (add `self.OnDestroyed` (`self.CurrentWeapon`) (delegate `RespawnWeapon`)))

(fn `UserConstructionScript`)